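; Save system test actor that holds counters as objects, static and dynamic components, arrays and nested structs.
; On authority, BeginPlay creates missing counters and spawns an attached child copy unless already attached, skipping all setup when BeforeLoad has set Loaded.
; Interact increments every counter, then after a short delay calls UpdateTextOnClients to show the counts on a TextRender.
; Save and load hooks print when they fire.
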(event `self.ReceiveBeginPlay`
  (bind (_returnvalue_location _returnvalue_rotation _returnvalue_scale) (`KismetMathLibrary.BreakTransform` (`self.GetTransform` self)))
  (`parent.ReceiveBeginPlay`)
  (`/Engine/EditorBlueprintResources/ActorMacros.Switch Has Authority`
    (:`Authority`
      (if (not (`self.bLoaded`))
        (`/Engine/EditorBlueprintResources/StandardMacros.IsValid` (`self.ObjectCounter`)
          (:`Is Valid`
            _)
          (:`Is Not Valid`
            (bind _returnvalue (`|GenericCreateObject` self "/Game/Blueprints/SaveSystem/BP_ObjectCounter.BP_ObjectCounter_C"))
            (set `self.ObjectCounter` _returnvalue)))
        (`/Engine/EditorBlueprintResources/StandardMacros.IsValid` (`self.DynamicEmbeddedCounter`)
          (:`Is Valid`
            _)
          (:`Is Not Valid`
            (bind _returnvalue_2 (`|AddComponentByClass` self "/Game/Blueprints/SaveSystem/BP_EmbeddedCounter.BP_EmbeddedCounter_C"))
            (set `self.DynamicEmbeddedCounter` _returnvalue_2)))
        (if (== (`KismetArrayLibrary.Array_Length` (`self.ArrayOfObjectCounters`)) 0)
          (for _ (range 2)
            (bind _returnvalue_3 (`|GenericCreateObject` self "/Game/Blueprints/SaveSystem/BP_ObjectCounter.BP_ObjectCounter_C"))
            (`KismetArrayLibrary.Array_Add` (`self.ArrayOfObjectCounters`) _returnvalue_3)))
        (`/Engine/EditorBlueprintResources/StandardMacros.IsValid` (`.Counter_3_B2E03E85451E7BDEF4DA43B89752AA81` (break `/Game/Blueprints/SaveSystem/SaveStructure` (`.SaveStructure_2_EC949FCB44369EE78EDDF6B450294ED2` (break `/Game/Blueprints/SaveSystem/SaveStructureWrap` (`self.Structure`)))))
          (:`Is Valid`
            _)
          (:`Is Not Valid`
            (bind _returnvalue_4 (`|GenericCreateObject` self "/Game/Blueprints/SaveSystem/BP_ObjectCounter.BP_ObjectCounter_C"))
            (set `self.Structure` (make `/Game/Blueprints/SaveSystem/SaveStructureWrap` (make `/Game/Blueprints/SaveSystem/SaveStructure` _returnvalue_4)))))
        (if (== (`KismetArrayLibrary.Array_Length` (`self.ArrayOfStructures`)) 0)
          (for _ (range 2)
            (bind _returnvalue_5 (`|GenericCreateObject` self "/Game/Blueprints/SaveSystem/BP_ObjectCounter.BP_ObjectCounter_C"))
            (`KismetArrayLibrary.Array_Add` (`self.ArrayOfStructures`) (make `/Game/Blueprints/SaveSystem/SaveStructureWrap` (make `/Game/Blueprints/SaveSystem/SaveStructure` _returnvalue_5)))))
        (if (not (`self.bAttached`))
          (bind _returnvalue_6 (`|SpawnActorFromClass` "BP_Counter_C" (`KismetMathLibrary.MakeTransform` (+ _returnvalue_location (0.0 0.0 100.0)) _returnvalue_rotation _returnvalue_scale) "AlwaysSpawn" "OverrideRootScale" null true null))
          (`self.K2_AttachToActor` _returnvalue_6 self "None" "KeepWorld" "KeepWorld" "KeepWorld" true))
        (`self.UpdateText`)))))

(event `Interact`
  (`/Engine/EditorBlueprintResources/StandardMacros.IncrementInt` (`/Game/Blueprints/SaveSystem/BP_ObjectCounter.Count` (`self.ObjectCounter`))
    (:`  `
      (`/Engine/EditorBlueprintResources/StandardMacros.IncrementInt` (`/Game/Blueprints/SaveSystem/BP_EmbeddedCounter.Count` (`self.BP_EmbeddedCounter`))
        (:`  `
          (`/Engine/EditorBlueprintResources/StandardMacros.IncrementInt` (`/Game/Blueprints/SaveSystem/BP_EmbeddedCounter.Count` (`self.DynamicEmbeddedCounter`))
            (:`  `
              (for _array_element (`self.ArrayOfObjectCounters`)
                (`/Engine/EditorBlueprintResources/StandardMacros.IncrementInt` (`/Game/Blueprints/SaveSystem/BP_ObjectCounter.Count` _array_element)))
              (`/Engine/EditorBlueprintResources/StandardMacros.IncrementInt` (`/Game/Blueprints/SaveSystem/BP_ObjectCounter.Count` (`.Counter_3_B2E03E85451E7BDEF4DA43B89752AA81` (break `/Game/Blueprints/SaveSystem/SaveStructure` (`.SaveStructure_2_EC949FCB44369EE78EDDF6B450294ED2` (break `/Game/Blueprints/SaveSystem/SaveStructureWrap` (`self.Structure`))))))
                (:`  `
                  (for _array_element_2 (`self.ArrayOfStructures`)
                    (`/Engine/EditorBlueprintResources/StandardMacros.IncrementInt` (`/Game/Blueprints/SaveSystem/BP_ObjectCounter.Count` (`.Counter_3_B2E03E85451E7BDEF4DA43B89752AA81` (break `/Game/Blueprints/SaveSystem/SaveStructure` (`.SaveStructure_2_EC949FCB44369EE78EDDF6B450294ED2` (break `/Game/Blueprints/SaveSystem/SaveStructureWrap` _array_element_2)))))))
                  (`KismetSystemLibrary.Delay` 0.5)
                  (`self.UpdateTextOnClients`))))))))))

(event `UpdateText`
  (`TextRenderComponent.K2_SetText` (`self.TextRender`) (`KismetTextLibrary.Conv_StringToText` (`KismetStringLibrary.Concat_StrStr` (`KismetStringLibrary.Conv_IntToString` (`/Game/Blueprints/SaveSystem/BP_ObjectCounter.Count` (`self.ObjectCounter`))) " " (`KismetStringLibrary.Conv_IntToString` (`/Game/Blueprints/SaveSystem/BP_EmbeddedCounter.Count` (`self.BP_EmbeddedCounter`))) " " (`KismetStringLibrary.Conv_IntToString` (`/Game/Blueprints/SaveSystem/BP_EmbeddedCounter.Count` (`self.DynamicEmbeddedCounter`))) " " (`KismetStringLibrary.Conv_IntToString` (`/Game/Blueprints/SaveSystem/BP_ObjectCounter.Count` (`|GetArrayItem` (`self.ArrayOfObjectCounters`)))) " " (`KismetStringLibrary.Conv_IntToString` (`/Game/Blueprints/SaveSystem/BP_ObjectCounter.Count` (`|GetArrayItem` (`self.ArrayOfObjectCounters`) 1))) " " (`KismetStringLibrary.Conv_IntToString` (`/Game/Blueprints/SaveSystem/BP_ObjectCounter.Count` (`.Counter_3_B2E03E85451E7BDEF4DA43B89752AA81` (break `/Game/Blueprints/SaveSystem/SaveStructure` (`.SaveStructure_2_EC949FCB44369EE78EDDF6B450294ED2` (break `/Game/Blueprints/SaveSystem/SaveStructureWrap` (`self.Structure`))))))) " " (`KismetStringLibrary.Conv_IntToString` (`/Game/Blueprints/SaveSystem/BP_ObjectCounter.Count` (`.Counter_3_B2E03E85451E7BDEF4DA43B89752AA81` (break `/Game/Blueprints/SaveSystem/SaveStructure` (`.SaveStructure_2_EC949FCB44369EE78EDDF6B450294ED2` (break `/Game/Blueprints/SaveSystem/SaveStructureWrap` (`|GetArrayItem` (`self.ArrayOfStructures`)))))))) " " (`KismetStringLibrary.Conv_IntToString` (`/Game/Blueprints/SaveSystem/BP_ObjectCounter.Count` (`.Counter_3_B2E03E85451E7BDEF4DA43B89752AA81` (break `/Game/Blueprints/SaveSystem/SaveStructure` (`.SaveStructure_2_EC949FCB44369EE78EDDF6B450294ED2` (break `/Game/Blueprints/SaveSystem/SaveStructureWrap` (`|GetArrayItem` (`self.ArrayOfStructures`) 1)))))))))))

(event `UpdateTextOnClients`
  (`self.UpdateText`))

(event `SaveableInterface.BeforeSave`
  (`KismetSystemLibrary.PrintString` "Actor: BeforeSave"))

(event `SaveableInterface.BeforeLoad`
  (`KismetSystemLibrary.PrintString` "Actor: BeforeLoad")
  (set `self.bLoaded` true))

(event `SaveableInterface.AfterSave`
  (`KismetSystemLibrary.PrintString` "Actor: AfterSave"))

(event `SaveableInterface.AfterLoad`
  (`KismetSystemLibrary.PrintString` "Actor: AfterLoad"))

(fn `UserConstructionScript`)