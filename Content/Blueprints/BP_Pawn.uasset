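; Player pawn that interacts with counters and provides keyboard-triggered save and load of saveable actors.
; F line-traces 300 units forward and calls Interact on a hit BP_Counter.
; N passes SaveableInterface actors without a valid attach parent to a PartialSaveGame and writes it to a slot.
; M destroys all SaveableInterface actors, then loads that slot and calls the save object's Load.
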(event `Key|F`
  (params (Key :type "Key Structure"))
  (bind _returnvalue (`self.K2_GetActorLocation`))
  (:`Pressed`
    (bind _outhit (`KismetSystemLibrary.LineTraceSingle` :`Start` _returnvalue :`End` (+ _returnvalue (* (`self.GetActorForwardVector`) 300.0)) :`TraceChannel` "TraceTypeQuery1" :`DrawDebugType` "ForDuration" :`DrawTime` 10.0))
    (bind _asbp_counter (cast `/Game/Blueprints/SaveSystem/BP_Counter` (`.HitActor` (`GameplayStatics.BreakHitResult` _outhit))))
    (`/Game/Blueprints/SaveSystem/BP_Counter.Interact` _asbp_counter)))

(event `Key|N`
  (params (Key :type "Key Structure"))
  (:`Pressed`
    (`self.SaveGame`)))

(event `SaveGame`
  (bind _outactors (`GameplayStatics.GetAllActorsWithInterface` "/Script/MySaveSystemPlugin.SaveableInterface"))
  (for _array_element _outactors
    (`/Engine/EditorBlueprintResources/StandardMacros.IsValid` (`self.GetAttachParentActor` _array_element)
      (:`Is Not Valid`
        (`KismetArrayLibrary.Array_Add` (`self.ActorsToSave`) _array_element))))
  (bind _returnvalue (`GameplayStatics.CreateSaveGameObject` "/Script/MySaveSystemPlugin.PartialSaveGame"))
  (`PartialSaveGame.Save` _returnvalue (`self.ActorsToSave`))
  (`GameplayStatics.SaveGameToSlot` _returnvalue "1"))

(event `Key|M`
  (params (Key :type "Key Structure"))
  (:`Pressed`
    (`self.LoadGame`)))

(event `LoadGame`
  (bind _outactors (`GameplayStatics.GetAllActorsWithInterface` "/Script/MySaveSystemPlugin.SaveableInterface"))
  (for _array_element _outactors
    (`self.K2_DestroyActor` _array_element))
  (bind _returnvalue (`GameplayStatics.LoadGameFromSlot` "1"))
  (bind _aspartial_save_game (cast `PartialSaveGame` _returnvalue))
  (`PartialSaveGame.Load` _aspartial_save_game))

(fn `UserConstructionScript`)